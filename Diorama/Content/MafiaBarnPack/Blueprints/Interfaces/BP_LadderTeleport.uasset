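; Interactable ladder actor that teleports the player character to a destination point instead of having them climb.
; A box overlap shows or hides an interact UI component while a character is inside.
; InteractCase fades the camera to black, moves and rotates the player to DestinationPoint, then fades back in.
; A DoOnce blocks repeat triggers until the sequence finishes.
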(event OnComponentBeginOverlap(Box)
  (params (OverlappedComponent :type Primitive%20Component%20Object%20Reference) (OtherActor :type Actor%20Object%20Reference) (OtherComp :type Primitive%20Component%20Object%20Reference) (OtherBodyIndex :type Integer) (bFromSweep :type Boolean) (SweepResult :type Hit%20Result%20Structure%20%28by%20ref%29))
  (Utilities|Casting|CastToCharacter OtherActor)
  (Rendering|SetVisibility (Variables|Default|GetInteractUI) true false))

(event OnComponentEndOverlap(Box)
  (params (OverlappedComponent :type Primitive%20Component%20Object%20Reference) (OtherActor :type Actor%20Object%20Reference) (OtherComp :type Primitive%20Component%20Object%20Reference) (OtherBodyIndex :type Integer))
  (Utilities|Casting|CastToCharacter OtherActor)
  (Rendering|SetVisibility (Variables|Default|GetInteractUI) false false))

(event EventBeginPlay
  (|CallParentFunction) ; This node is disabled and will not be called.\nDrag off pins to build functionality.
)

(event Collision|EventActorBeginOverlap
  (params (OtherActor :type Actor%20Object%20Reference))
  (|CallParentFunction OtherActor) ; This node is disabled and will not be called.\nDrag off pins to build functionality.
)

(event EventTick
  (params (DeltaSeconds :type Float%20%28single-precision%29))
  (|CallParentFunction DeltaSeconds) ; This node is disabled and will not be called.\nDrag off pins to build functionality.
)

(event EventInteractCase
  (bind _destinationpoint (Variables|Default|GetDestinationPoint))
  (Utilities|FlowControl|DoOnce false :!label _label
    (:Completed
      (CameraFades|StartCameraFade :self (Game|GetPlayerCameraManager 0) :ToAlpha 1.0 :Duration 1.0 :bHoldWhenFinished true)
      (Utilities|FlowControl|Delay 1.0)
      (Transformation|SetActorLocationAndRotation (Game|GetPlayerCharacter 0) (Transformation|GetWorldLocation _destinationpoint) (Transformation|GetWorldRotation _destinationpoint))
      (Utilities|FlowControl|Delay 0.5)
      (CameraFades|StartCameraFade :self (Game|GetPlayerCameraManager 0) :FromAlpha 1.0 :Duration 1.0)
      (goto _label Reset))))

(fn ConstructionScript
  (|CallParentFunction))